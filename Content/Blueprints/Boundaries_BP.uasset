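; Boundary actor that warns either of two players through AlertHUD when they enter an out-of-map zone.
; Begin overlap flags the TestFX_Player as in boundaries and starts the P1 or P2 alert timer by OtherPlayerIndex; end overlap clears it and hides that alert.
; A TwoOverlapp flag covers a second simultaneous overlap, so the alert persists until the player leaves both.
; Tick is empty, leaving a widget-removal fallback unconnected.
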(event EventTick
  (params (DeltaSeconds :type Float%20%28single-precision%29))
  ;[1 1 1] Si jamais ca a pas le temps de remove
)

(event Collision|EventActorBeginOverlap
  (params (OtherActor :type Actor%20Object%20Reference))
  (bind _alerthud (Variables|Default|GetAlertHUD))
  ;[1 1 1] Widget sortie map
  (bind _astest_fx_player (Utilities|Casting|CastToTestFX_Player OtherActor))
  (if (Variables|/Game/Blueprints/TestFX_Player.TestFX_Player_C|GetIsInBoundaries _astest_fx_player)
    (Variables|/Game/Blueprints/TestFX_Player.TestFX_Player_C|SetTwoOverlapp _astest_fx_player true)
    (else
      (Variables|/Game/Blueprints/TestFX_Player.TestFX_Player_C|SetIsInBoundaries _astest_fx_player true)
      (if (== (Variables|/Game/Blueprints/TestFX_Player.TestFX_Player_C|GetOtherPlayerIndex _astest_fx_player) 1)
        (Default|P1TimerEvent _alerthud)
        (else
          (Default|P2TimerEvent _alerthud))))))

(event Collision|EventActorEndOverlap
  (params (OtherActor :type Actor%20Object%20Reference))
  (bind _alerthud (Variables|Default|GetAlertHUD))
  (bind _astest_fx_player (Utilities|Casting|CastToTestFX_Player OtherActor))
  (if (Variables|/Game/Blueprints/TestFX_Player.TestFX_Player_C|GetTwoOverlapp _astest_fx_player)
    (Variables|/Game/Blueprints/TestFX_Player.TestFX_Player_C|SetTwoOverlapp _astest_fx_player false)
    (else
      (Variables|/Game/Blueprints/TestFX_Player.TestFX_Player_C|SetIsInBoundaries _astest_fx_player false)
      (if (== (Variables|/Game/Blueprints/TestFX_Player.TestFX_Player_C|GetOtherPlayerIndex _astest_fx_player) 1)
        (Default|HideP1Alert _alerthud)
        (else
          (Default|HideP2Alert _alerthud))))))

(fn ConstructionScript)