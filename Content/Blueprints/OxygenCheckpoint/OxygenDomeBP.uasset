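; Oxygen dome checkpoint that sets the player's respawn point and restores their energy while they are inside.
; On BeginPlay it takes a random starting yaw, which a timeline then offsets to rotate the whole actor.
; Entering the dome saves its location for respawn, plays a regen sound, calls the HUD's oxygen check and starts a fast looping RestoreEnergy timer on the player.
; Leaving the dome clears that timer.
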(event OnComponentBeginOverlap(OxDome)
  (params (OverlappedComponent :type Primitive%20Component%20Object%20Reference) (OtherActor :type Actor%20Object%20Reference) (OtherComp :type Primitive%20Component%20Object%20Reference) (OtherBodyIndex :type Integer) (bFromSweep :type Boolean) (SweepResult :type Hit%20Result%20Structure%20%28by%20ref%29))
  (bind _astest_fx_player (Utilities|Casting|CastToTestFX_Player OtherActor))
  (Variables|/Game/Blueprints/TestFX_Player.TestFX_Player_C|SetRespawnLocation _astest_fx_player (Transformation|GetActorLocation))
  (Audio|PlaySound2D "/Game/SFX/RegenOxygen_Cue.RegenOxygen_Cue" 1.0 1.0 0.0 0 0)
  (Default|CheckOxygen (Variables|/Game/Blueprints/TestFX_Player.TestFX_Player_C|GetHUD%20Player _astest_fx_player))
  (Utilities|Time|SetTimerbyFunctionName _astest_fx_player "RestoreEnergy" 0.01 true))

(event OnComponentEndOverlap(OxDome)
  (params (OverlappedComponent :type Primitive%20Component%20Object%20Reference) (OtherActor :type Actor%20Object%20Reference) (OtherComp :type Primitive%20Component%20Object%20Reference) (OtherBodyIndex :type Integer))
  (bind _astest_fx_player (Utilities|Casting|CastToTestFX_Player OtherActor))
  (Utilities|Time|ClearTimerbyFunctionName _astest_fx_player "RestoreEnergy"))

(event EventBeginPlay
  (bind _output_get (Variables|Default|SetInitRotation (Math|Random|RandomFloatinRange 0.0 3.6e+02)))
  (Transformation|SetActorRelativeRotation (Math|Rotator|MakeRotator 0.0 0.0 _output_get))
  (bind _rotation (Timeline|AsteroidRotation PlayFromStart)
    (:Update
      (Transformation|SetActorRelativeRotation (Math|Rotator|MakeRotator 0.0 0.0 (+ _rotation (Variables|Default|GetInitRotation)))))))

(fn ConstructionScript)