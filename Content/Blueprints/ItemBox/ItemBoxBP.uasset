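; Item box pickup that floats and spins on a timeline and grants a random item to an overlapping TestFX_Player.
; The overlap sets the player's item, then hides and updates the power-up display on PowerUpHUD for player one or two, chosen by OtherPlayerIndex.
; PoppedEvent then toggles the box's visibility and disables collision, restoring both after a short delay, with a Popped flag blocking repeat pickups meanwhile.
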(event OnComponentBeginOverlap(ItemBox)
  (params (OverlappedComponent :type Primitive%20Component%20Object%20Reference) (OtherActor :type Actor%20Object%20Reference) (OtherComp :type Primitive%20Component%20Object%20Reference) (OtherBodyIndex :type Integer) (bFromSweep :type Boolean) (SweepResult :type Hit%20Result%20Structure%20%28by%20ref%29))
  (bind _poweruphud (Variables|Default|GetPowerUpHUD))
  (bind _astest_fx_player (Utilities|Casting|CastToTestFX_Player OtherActor))
  (if (not (Variables|Default|GetPopped))
    (bind _output_get (Variables|/Game/Blueprints/TestFX_Player.TestFX_Player_C|SetItem _astest_fx_player (Math|Random|RandomIntegerinRange 1 9)))
    (CallFunction|HidePowerUp (Variables|/Game/Blueprints/TestFX_Player.TestFX_Player_C|GetOtherPlayerIndex _astest_fx_player))
    (if (== (Variables|/Game/Blueprints/TestFX_Player.TestFX_Player_C|GetOtherPlayerIndex _astest_fx_player) 1)
      (Default|P1PowerUp _poweruphud _output_get)
      (else
        (Default|P2PowerUp _poweruphud _output_get)))
    (CallFunction|PoppedEvent)))

(event Custom|PoppedEvent
  (bind _itembox (Variables|Default|GetItemBox))
  (Variables|Default|SetPopped true)
  (Rendering|ToggleVisibility _itembox false)
  (Collision|SetCollisionEnabled _itembox "NoCollision")
  (Utilities|FlowControl|Delay 2.5)
  (Rendering|ToggleVisibility _itembox false)
  (Collision|SetCollisionEnabled _itembox "QueryAndPhysics")
  (Variables|Default|SetPopped false))

(event EventBeginPlay
  (bind (_direction _rotation _foating) (Timeline|Movement PlayFromStart)
    (:Update
      (Transformation|SetRelativeLocationAndRotation (Variables|Default|GetItemBox) (Math|Vector|MakeVector 0.0 0.0 _foating) (Math|Rotator|MakeRotator 0.0 0.0 _rotation) false false))))

(event Collision|EventActorBeginOverlap
  (params (OtherActor :type Actor%20Object%20Reference)))

(event EventTick
  (params (DeltaSeconds :type Float%20%28single-precision%29)))

(fn ConstructionScript)

(fn HidePowerUp
  (params (OtherPlay :type Integer))
  (bind _poweruphud (Variables|Default|GetPowerUpHUD))
  (if (== OtherPlay 1)
    (Default|HideP1PowerUp _poweruphud)
    (else
      (Default|HideP2PowerUp _poweruphud))))