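; Shared camera for a two-player race-style game that follows both TestFX_Player actors and ends the round when one leaves the screen.
; Each tick it centers between the players, biases toward the leader using the Winning flag, and scales the offset and spring arm length with their separation.
; After a one-second startup delay, an unrendered player triggers hiding the Winner (set by P1Win/P2Win), moving them to Finish and switching their view there.
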(event Custom|P2Win
  (Variables|Default|SetWinner 1))

(event Custom|P1Win
  (Variables|Default|SetWinner 0))

(event EventBeginPlay
  (bind _outactors (Actor|GetAllActorsOfClass "/Game/Blueprints/TestFX_Player.TestFX_Player_C"))
  (Variables|Default|SetPlayers _outactors)
  (Game|Player|SetViewTargetwithBlend (Game|GetPlayerController 0) self 0.0 "VTBlend_Linear" 0.0 false)
  (Utilities|FlowControl|Delay 1.0)
  (Variables|Default|SetStarted true))

(event EventTick
  (params (DeltaSeconds :type Float%20%28single-precision%29))
  (bind _defaultsceneroot (Variables|Default|GetDefaultSceneRoot))
  (bind _players (Variables|Default|GetPlayers))
  (bind _players_2 (Variables|Default|GetPlayers))
  (bind _winner (Variables|Default|GetWinner))
  (bind _returnvalue (Game|GetPlayerCharacter _winner))
  (bind _output (Utilities|Array|Get(acopy) _players_2))
  (bind _output_2 (Utilities|Array|Get(acopy) _players_2 1))
  (bind _output_3 (Utilities|Array|Get(acopy) _players))
  (bind _output_4 (Utilities|Array|Get(acopy) _players 1))
  (bind _returnvalue_2 (Class|GameplayStatics|GetActorArrayAverageLocation (Variables|Default|GetPlayers)))
  (Variables|Default|SetDistanceFollowing (Math|Float|MapRangeClamped (Transformation|GetDistanceTo _output _output_2) 5e+02 2e+03 0.0 0.5))
  (if (Variables|/Game/Blueprints/TestFX_Player.TestFX_Player_C|GetWinning _output)
    (Transformation|SetWorldLocation _defaultsceneroot (+ _returnvalue_2 (* (* (- (Transformation|GetActorLocation _output) (Transformation|GetActorLocation _output_2)) (Variables|Default|GetDistanceFollowing)) 0.75)) false false)
    (else
      (Transformation|SetWorldLocation _defaultsceneroot (+ _returnvalue_2 (* (* (- (Transformation|GetActorLocation _output) (Transformation|GetActorLocation _output_2)) (Variables|Default|GetDistanceFollowing)) -0.75)) false false)))
  (Variables|/Script/Engine.SpringArmComponent|SetTargetArmLength (Variables|Default|GetSpringArm) (Math|Float|MapRangeClamped (Transformation|GetDistanceTo _output_3 _output_4) 0.0 1.5e+03 3e+02 4e+03))
  (if (Variables|Default|GetStarted)
    (if (not (and (Class|Actor|WasRecentlyRendered _output_3 0.1) (Class|Actor|WasRecentlyRendered _output_4 0.1)))
      (Rendering|SetActorHiddenInGame _returnvalue true)
      (Transformation|SetActorLocation _returnvalue (Transformation|GetWorldLocation (Variables|/Script/Engine.Actor|GetRootComponent (Variables|Default|Getfinish))) false false)
      (Game|Player|SetViewTargetwithBlend (Game|GetPlayerController (Variables|Default|GetWinner)) (Variables|Default|Getfinish) 0.0 "VTBlend_Linear" 0.0 false))))

(fn ConstructionScript)