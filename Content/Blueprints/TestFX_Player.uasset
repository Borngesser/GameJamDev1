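; Two-player character that moves by dashing along an arrow, spending oxygen energy, and can respawn at its start point.
; A timeline spins the arrow, or axis input aims it in ModeRemi, while mesh spin rate scales with velocity.
; Held items alter either player's arrow, dash or energy, or trigger stun, shield or a timer-driven grapple pulling both players together.
; The shield blocks only stun and grapple; construction picks mesh and AnimBP from OtherPlayerIndex.
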(event Custom|Respawn
  (bind _respawnlocation (Variables|Default|GetRespawnLocation))
  ;[1 1 1] Respawn
  (Transformation|SetActorLocation (Math|Vector|MakeVector (.x _respawnlocation) (.y _respawnlocation) 14.0) false false)
  (Utilities|FlowControl|Delay 0.1)
  (Components|Movement|StopMovementImmediately (Variables|Character|GetCharacterMovement))
  (Variables|Default|SetCurrentEnergy 1e+03)
  (Default|CheckOxygen (Variables|Default|GetHUD%20Player)))

(event Custom|RotateMeshWithVelocity
  ;[1 1 1] Rotate Mesh With Velocity
  (Components|Timeline|SetPlayRate (Variables|Default|GetMeshRotation) (Math|Float|MapRangeClamped (Math|Float|MapRangeClamped (Math|Vector|VectorLength (Transformation|GetVelocity)) 0.0 6e+02 9e+01 3.6e+02) 9e+01 4e+02 1.0 6.0)))

(event EventTick
  (params (DeltaSeconds :type Float%20%28single-precision%29))
  (bind _asgame_instance_projet (Utilities|Casting|CastToGameInstanceProjet (Game|GetGameInstance)))
  (if (Variables|/Game/Blueprints/GameInstanceProjet.GameInstanceProjet_C|GetModeRemi _asgame_instance_projet)
    (Transformation|SetWorldRotation (Variables|Default|GetArrow_) (Math|Rotator|MakeRotator 0.0 0.0 (+ (.yaw (Math|Conversions|RotationFromXVector (Math|Vector|MakeVector (Input|AxisValues|GetRotateRemiX) (Input|AxisValues|GetRotateRemiY) 0.0))) 9e+01)) false false)))

(event EventBeginPlay
  (Utilities|FlowControl|Sequence
    (:then_0
      ;[1 1 1] Initial Spawn
      (Variables|Default|SetRespawnLocation (Transformation|GetActorLocation)))
    (:then_1
      ;[1 1 1] Arrow Movement
      (bind _asgame_instance_projet (Utilities|Casting|CastToGameInstanceProjet (Game|GetGameInstance)))
      (if (not (Variables|/Game/Blueprints/GameInstanceProjet.GameInstanceProjet_C|GetModeRemi _asgame_instance_projet))
        (bind _rotation (Timeline|AnimArrow PlayFromStart)
          (:Update
            (Transformation|SetRelativeRotation (Variables|Default|GetArrow_) (Math|Rotator|MakeRotator 0.0 0.0 _rotation) false false)))))
    (:then_2
      (Utilities|FlowControl|Sequence
        (:then_0
          ;[1 1 1] Random Mesh Rotation at begin
          (Variables|Default|SetRandomMeshRotation (Math|Random|RandomFloatinRange 0.0 3.6e+02))
          (bind _rotation_2 (Timeline|MeshRotation PlayFromStart)
            (:Update
              (Transformation|SetRelativeRotation (Variables|Character|GetMesh) (Math|Rotator|MakeRotator -9e+01 0.0 (+ _rotation_2 (Variables|Default|GetRandomMeshRotation))) false false))))
        (:then_1
          ;[1 1 1] Rotate Mesh With Velocity
          (Utilities|Time|SetTimerbyEvent (delegate Custom|RotateMeshWithVelocity) 0.01 true))))))

(event Input|ActionEvents|InputActionDash
  (params (Key :type Key%20Structure :default "None"))
  (bind _arrow_ (Variables|Default|GetArrow_))
  (bind _returnvalue (Math|Vector|GetForwardVector _arrow_))
  ;[1 1 1] Dash
  (:Pressed
    (if (> (Variables|Default|GetCurrentEnergy) 0.0)
      (Audio|PlaySound2D "/Game/SFX/Dash_Oxygen_Cue.Dash_Oxygen_Cue" 1.0 1.0 0.0 0 0)
      (Character|LaunchCharacter (* (* (Math|Vector|MakeVector (.x _returnvalue) (.y _returnvalue) 0.0) 5e+02) (Variables|Default|GetDashType)) false false)
      (if (not (== (Variables|Default|GetDashType) 0))
        (Variables|Default|SetCurrentEnergy (- (Variables|Default|GetCurrentEnergy) 1e+02))
        (Default|CheckOxygen (Variables|Default|GetHUD%20Player)))
      (else
        (Audio|PlaySound2D "/Game/SFX/empty.empty" 1.0 1.0 0.0 0 0)))))

(event Input|ActionEvents|InputActionRespawn
  (params (Key :type Key%20Structure :default "None"))
  ;[1 1 1] Respawn
  (:Pressed
    (if (not (Variables|Default|GetGrappled))
      (CallFunction|Respawn))))

(event Custom|DeactivateShield
  ;[1 1 1] Deactivate Shield
  (Variables|Default|SetShieldOn false)
  (Rendering|ToggleVisibility (Variables|Default|GetShield) false))

(event Custom|Stun
  (bind _stunned (Variables|Default|GetStunned))
  (bind _arrow_ (Variables|Default|GetArrow_))
  (bind _animarrow (Variables|Default|GetAnimArrow))
  ;[1 1 1] Stun Event
  (if (not (Variables|Default|GetShieldOn))
    (Components|Timeline|SetPlayRate _animarrow 0.0)
    (Components|Activation|SetActive _stunned true false)
    (Rendering|Material|SetVectorParameterValueonMaterials _arrow_ "BaseColor" "0, 0, 0")
    (Variables|Default|SetDashType 0)
    (Utilities|FlowControl|Delay 3.0)
    (Components|Activation|SetActive _stunned false false)
    (Components|Timeline|SetPlayRate _animarrow 1.0)
    (Rendering|Material|SetVectorParameterValueonMaterials _arrow_ "BaseColor" "1.000000,0.000000,0.000000")
    (Variables|Default|SetDashType 1)
    (else
      (CallFunction|DeactivateShield))))

(event Input|ActionEvents|InputActionPowerUp
  (params (Key :type Key%20Structure))
  (bind _otherplayerindex (Variables|Default|GetOtherPlayerIndex))
  (bind _otherplayerindex_2 (Variables|Default|GetOtherPlayerIndex))
  (bind _otherplayerindex_3 (Variables|Default|GetOtherPlayerIndex))
  (bind _otherplayerindex_4 (Variables|Default|GetOtherPlayerIndex))
  (bind _animarrow (Variables|Default|GetAnimArrow))
  (bind _otherplayerindex_5 (Variables|Default|GetOtherPlayerIndex))
  (bind _otherplayerindex_6 (Variables|Default|GetOtherPlayerIndex))
  (bind _returnvalue (Game|GetPlayerCharacter _otherplayerindex_6))
  (bind _returnvalue_2 (Game|GetPlayerCharacter _otherplayerindex_2))
  (bind _returnvalue_3 (Game|GetPlayerCharacter _otherplayerindex_4))
  (bind _returnvalue_4 (Game|GetPlayerCharacter _otherplayerindex))
  (bind _returnvalue_5 (Game|GetPlayerCharacter _otherplayerindex_3))
  (bind _returnvalue_6 (Game|GetPlayerCharacter _otherplayerindex_5))
  (bind _astest_fx_player (Utilities|Casting|CastToTestFX_Player _returnvalue_5))
  (bind _astest_fx_player_2 (Utilities|Casting|CastToTestFX_Player _returnvalue_3))
  (bind _astest_fx_player_3 (Utilities|Casting|CastToTestFX_Player _returnvalue))
  (bind _astest_fx_player_4 (Utilities|Casting|CastToTestFX_Player _returnvalue_2))
  (bind _astest_fx_player_5 (Utilities|Casting|CastToTestFX_Player _returnvalue_4))
  (bind _astest_fx_player_6 (Utilities|Casting|CastToTestFX_Player _returnvalue_6))
  (bind _arrow_ (Variables|TestFX_Player_C|GetArrow_ _astest_fx_player_4))
  (bind _animarrow_2 (Variables|TestFX_Player_C|GetAnimArrow _astest_fx_player_5))
  (bind _animarrow_3 (Variables|TestFX_Player_C|GetAnimArrow _astest_fx_player_6))
  (:Pressed
    (bind _returnvalue_7 (Actor|GetActorOfClass "/Game/Blueprints/ItemBox/ItemBoxBP.ItemBoxBP_C"))
    (Default|HidePowerUp _returnvalue_7 (Variables|Default|GetOtherPlayerIndex))
    (switch int (Variables|Default|GetItem)
      (:0
        (Development|PrintString "No Item"))
      (:1
        ;[1 1 1] Accélération Flèche
        (Variables|Default|SetItem 0)
        (Components|Timeline|SetPlayRate _animarrow_2 2.0)
        (Utilities|FlowControl|Delay 1e+01)
        (Components|Timeline|SetPlayRate _animarrow_2 1.0))
      (:2
        ;[1 1 1] Ralentissement Flèche
        (Variables|Default|SetItem 0)
        (Components|Timeline|SetPlayRate _animarrow 0.5)
        (Utilities|FlowControl|Delay 1e+01)
        (Components|Timeline|SetPlayRate _animarrow 1.0))
      (:3
        ;[1 1 1] Inversement Dash
        (Variables|Default|SetItem 0)
        (Rendering|Material|SetVectorParameterValueonMaterials _arrow_ "BaseColor" "0.000000,0.000000,1.000000")
        (Variables|TestFX_Player_C|SetDashType _astest_fx_player_4 -1)
        (Utilities|FlowControl|Delay 1e+01)
        (Variables|TestFX_Player_C|SetDashType _astest_fx_player_4 1)
        (Rendering|Material|SetVectorParameterValueonMaterials _arrow_ "BaseColor" "1.000000,0.000000,0.000000"))
      (:4
        ;[1 1 1] Inversement Flèche
        (Variables|Default|SetItem 0)
        (Components|Timeline|SetPlayRate _animarrow_3 -1.0)
        (Utilities|FlowControl|Delay 1e+01)
        (Components|Timeline|SetPlayRate _animarrow_3 1.0))
      (:5
        ;[1 1 1] Stun
        (Variables|Default|SetItem 0)
        (CallFunction|Stun (.AsTest%20FX%20Player (Utilities|Casting|CastToTestFX_Player (Game|GetPlayerCharacter (Variables|Default|GetOtherPlayerIndex))))))
      (:6
        ;[1 1 1] Voler Energie
        (Variables|Default|SetItem 0)
        (if (< (Variables|TestFX_Player_C|GetCurrentEnergy _astest_fx_player) 2.5e+02)
          (if (> (Variables|TestFX_Player_C|GetCurrentEnergy _astest_fx_player) 0.0)
            (Variables|Default|SetCurrentEnergy (+ (Variables|Default|GetCurrentEnergy) (Variables|TestFX_Player_C|GetCurrentEnergy _astest_fx_player)))
            (Variables|TestFX_Player_C|SetCurrentEnergy _astest_fx_player 0.0)
            (Default|CheckOxygen (Variables|Default|GetHUD%20Player))
            (else
              (Default|CheckOxygen (Variables|Default|GetHUD%20Player) :!label _label)))
          (else
            (Variables|Default|SetCurrentEnergy (+ (Variables|Default|GetCurrentEnergy) 2.5e+02))
            (Variables|TestFX_Player_C|SetCurrentEnergy _astest_fx_player (- (Variables|TestFX_Player_C|GetCurrentEnergy _astest_fx_player) 2.5e+02))
            (goto _label))))
      (:7
        ;[1 1 1] Perdre Energie
        (Variables|Default|SetItem 0)
        (Variables|TestFX_Player_C|SetCurrentEnergy _astest_fx_player_2 (- (Variables|TestFX_Player_C|GetCurrentEnergy _astest_fx_player_2) 5e+02))
        (if (< (Variables|TestFX_Player_C|GetCurrentEnergy _astest_fx_player_2) 0.0)
          (Variables|TestFX_Player_C|SetCurrentEnergy _astest_fx_player_2 0.0))
        (Default|CheckOxygen (Variables|Default|GetHUD%20Player)))
      (:8
        ;[1 1 1] Activate Shield
        (Variables|Default|SetItem 0)
        (Variables|Default|SetShieldOn true)
        (Rendering|ToggleVisibility (Variables|Default|GetShield) false))
      (:9
        ;[1 1 1] Grapple
        (Variables|Default|SetItem 0)
        (if (not (Variables|TestFX_Player_C|GetShieldOn _astest_fx_player_3))
          (Collision|LineTraceByChannel (Transformation|GetActorLocation) (Transformation|GetActorLocation _astest_fx_player_3) "TraceTypeQuery1" false 0 "None")
          (Utilities|FlowControl|Sequence
            (:then_0
              (Utilities|Time|SetTimerbyFunctionName 0 "Grapple" 0.01 true)
              (bind _opacity (Timeline|GrappleOpacity PlayFromStart)
                (:Update
                  (Rendering|Material|SetScalarParameterValueonMaterials (Variables|Default|GetRope) "Opacity" _opacity))
                (:Finished
                  (Variables|Default|SetGrappled false))))
            (:then_1
              (Variables|Default|SetGrappled true)))
          (else
            (CallFunction|DeactivateShield _astest_fx_player_3)))))))

(fn ConstructionScript
  (bind _mesh (Variables|Character|GetMesh))
  (bind _mesh_2 (Variables|Character|GetMesh))
  (switch int (Variables|Default|GetOtherPlayerIndex)
    (:0
      ;[1 1 1] J2
      (Development|PrintString "J2")
      (Class|SkinnedMeshComponent|SetSkeletalMesh _mesh_2 "/Game/MixamoPlayer/Player_02/Player_02.Player_02" true)
      (Class|SkeletalMeshComponent|SetAnimClass _mesh_2 "/Game/MixamoPlayer/Player_02/Animation/AnimBP_Player02.AnimBP_Player02_C"))
    (:1
      ;[1 1 1] J1
      (Development|PrintString "J1")
      (Class|SkinnedMeshComponent|SetSkeletalMesh _mesh "/Game/MixamoPlayer/Player_01/Player_01.Player_01" true)
      (Class|SkeletalMeshComponent|SetAnimClass _mesh "/Game/MixamoPlayer/Player_01/Animation/AnimBp_Player01.AnimBp_Player01_C"))))

(fn Grapple
  (bind _returnvalue (Transformation|GetActorLocation))
  (bind _otherplayerindex (Variables|Default|GetOtherPlayerIndex))
  (bind _returnvalue_2 (Game|GetPlayerCharacter _otherplayerindex))
  (bind _astest_fx_player (Utilities|Casting|CastToTestFX_Player _returnvalue_2))
  (bind _returnvalue_3 (Transformation|GetActorLocation _astest_fx_player))
  (bind _returnvalue_4 (- _returnvalue_3 _returnvalue))
  (Utilities|FlowControl|Sequence
    (:then_0
      (if (not (Variables|Default|GetGrappled))
        (Utilities|Time|ClearTimerbyFunctionName 0 "Grapple")))
    (:then_1
      (Character|LaunchCharacter (/ _returnvalue_4 2) true false)
      (Character|LaunchCharacter _astest_fx_player (/ (- _returnvalue _returnvalue_3) 5) true false)
      (Variables|/Script/CableComponent.CableComponent|SetEndLocation (Variables|Default|GetRope) _returnvalue_4))))

(fn RestoreEnergy
  (if (< (Variables|Default|GetCurrentEnergy) 1e+03)
    (Variables|Default|SetCurrentEnergy (+ (Variables|Default|GetCurrentEnergy) 5.0))))