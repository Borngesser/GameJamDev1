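; Finish-line actor that ends the game when a TestFX_Player overlaps it and plays a spaceship getaway.
; The overlap swaps the HUD for a Win_Widget, naming J1 or J2 as survivor from the player's OtherPlayerIndex.
; It switches player 0's view to this actor, hides the box and runs a timeline moving the spaceship in X and Z from the start location.
; The mouse cursor appears when the timeline finishes.
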(event EventBeginPlay
  (Variables|Default|Setstartloc (Transformation|GetActorLocation)))

(event Collision|EventActorBeginOverlap
  (params (OtherActor :type Actor%20Object%20Reference))
  (bind _startloc (Variables|Default|Getstartloc))
  (bind _astest_fx_player (Utilities|Casting|CastToTestFX_Player OtherActor))
  (bind _returnvalue (UserInterface|CreateWidget "/Game/Widget/Win_Widget.Win_Widget_C" (Game|GetPlayerController 0)))
  (UserInterface|Viewport|AddtoViewport _returnvalue 0)
  (Widget|RemovefromParent (Variables|Default|GetHUD))
  (if (== (Variables|/Game/Blueprints/TestFX_Player.TestFX_Player_C|GetOtherPlayerIndex _astest_fx_player) 0)
    (Variables|/Game/Widget/Win_Widget.Win_Widget_C|Setwintext _returnvalue "J2 Survived !")
    (else
      (Variables|/Game/Widget/Win_Widget.Win_Widget_C|Setwintext _returnvalue "J1 Survived !")))
  (Game|Player|SetViewTargetwithBlend (Game|GetPlayerController 0) self 0.0 "VTBlend_Linear" 0.0 false)
  (Development|SetHiddeninGame (Variables|Default|GetBox) true false)
  (bind _newtrack_0 (Timeline|vaisseau%20qui%20ce%20barre Play)
    (:Update
      (Transformation|SetWorldLocation (Variables|Default|GetSpaceship) (Math|Vector|MakeVector (+ (.x _newtrack_0) (.x _startloc)) (.y _startloc) (+ (.z _startloc) (.z _newtrack_0))) false false))
    (:Finished
      (Variables|/Script/Engine.PlayerController|SetbShowMouseCursor (Game|GetPlayerController 0) true))))

(event EventTick
  (params (DeltaSeconds :type Float%20%28single-precision%29)))

(fn ConstructionScript)