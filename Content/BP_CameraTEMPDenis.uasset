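; Temporary shared camera for two TestFX_Player actors that becomes player 0's view target on BeginPlay.
; Each tick it moves its root to the players' average location and scales spring arm length with the distance between the first two, using a clamped range.
; Unconnected leftover logic checks whether either player was recently rendered, including a switch of view and position to a Finish actor when one is not.
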(event EventBeginPlay
  (bind _outactors (Actor|GetAllActorsOfClass "/Game/TopDownBP/Blueprints/TestFX_Player.TestFX_Player_C"))
  (Variables|Default|SetPlayers _outactors)
  (Game|Player|SetViewTargetwithBlend (Game|GetPlayerController 0) self 0.0 "VTBlend_Linear" 0.0 false))

(event EventTick
  (params (DeltaSeconds :type Float%20%28single-precision%29))
  (bind _players (Variables|Default|GetPlayers))
  (bind _returnvalue (Class|GameplayStatics|GetActorArrayAverageLocation (Variables|Default|GetPlayers)))
  (Transformation|SetWorldLocation (Variables|Default|GetDefaultSceneRoot) _returnvalue false false)
  (Variables|/Script/Engine.SpringArmComponent|SetTargetArmLength (Variables|Default|GetSpringArm) (Math|Float|MapRangeClamped (Transformation|GetDistanceTo (Utilities|Array|Get(acopy) _players) (Utilities|Array|Get(acopy) _players 1)) 0.0 1e+03 1e+03 2e+03)))

(fn ConstructionScript)